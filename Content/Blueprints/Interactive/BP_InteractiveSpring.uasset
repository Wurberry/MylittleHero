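; Interactive spring Blueprint that launches the player vertically when its Interact function is called.
; Interact launches the passed player with LaunchPower, overriding current Z velocity, and replays the Paper2D flipbook from the start.
; The construction script ties flipbook looping to the AutoPlay flag, and the event graph holds no active logic.
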(event EventBeginPlay
  (|CallParentFunction) ; This node is disabled and will not be called.\nDrag off pins to build functionality.
)

(event Collision|EventActorBeginOverlap
  (params (OtherActor :type Actor%20Object%20Reference)))

(event EventTick
  (params (DeltaSeconds :type Float%20%28single-precision%29)))

(fn ConstructionScript
  (Components|Timeline|SetLooping (Variables|Default|GetPaperFlipbook) (Variables|Default|GetbAutoPlay)))

(fn Interact
  (params (PlayerRef :type BP%20Player%20Base%20Object%20Reference))
  (Character|LaunchCharacter PlayerRef (Math|Vector|MakeVector 0.0 0.0 (Variables|Default|GetLaunchPower)) false true)
  (Components|Timeline|PlayfromStart (Variables|Default|GetPaperFlipbook)))