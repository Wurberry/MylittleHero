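; Interactive 2D checkpoint flag that acts as a level exit, saving progress and sending the player to the next level.
; Interact plays the flag-out flipbook once, and Tick switches to the idle flipbook when it finishes.
; Player overlap, independent of that used state, raises the unlocked level count in MainGameInstance and saves.
; A delayed transition then shows the loading screen and opens the next level in world 0.
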(event EventTick
  (params (DeltaSeconds :type Float%20%28single-precision%29))
  (bind _paperflipbook (Variables|Default|GetPaperFlipbook))
  ;[1 1 1] Control Animation
  (if (Variables|Default|GetbeUsed)
    (if (not (Audio|Components|Audio|IsPlaying (Variables|Default|GetPaperFlipbook)))
      (Components|Timeline|SetLooping _paperflipbook (Variables|Default|GetbAutoPlay))
      (Sprite|SetFlipbook _paperflipbook "/Game/Assets/Flipbooks/Checkpoint_Flag_IdleFlip.Checkpoint_Flag_IdleFlip")
      (Components|Timeline|PlayfromStart (Variables|Default|GetPaperFlipbook)))))

(event Collision|EventActorBeginOverlap
  (params (OtherActor :type Actor%20Object%20Reference))
  ;[1 1 1] Control Lvl Saved|Opened
  (if (== OtherActor (Game|GetPlayerCharacter 0))
    (bind _returnvalue (Game|GetCurrentLevelName true))
    (bind _lvlnum (Default|GetWrldLevelfromName (Variables|References|GetGameInstanceRef) _returnvalue))
    (Utilities|FlowControl|Sequence
      (:then_0
        (CallFunction|SetUnlockLevels (+ 1 _lvlnum))
        (Default|SaveGametoSlot (Variables|References|GetGameInstanceRef)))
      (:then_1
        (Utilities|BetweenTransferLevel
          (:Completed
            (Default|OpenLevel (Variables|References|GetGameInstanceRef) 0 (- (Variables|Default|GetnextLvlNumb) 1))))))))

(event EventBeginPlay
  ;[1 1 1] Create Game Inst Reference
  (bind _asmain_game_instance (Utilities|Casting|CastToMainGameInstance (Game|GetGameInstance)))
  (Variables|References|SetGameInstanceRef _asmain_game_instance))

(fn ConstructionScript
  (Components|Timeline|SetLooping (Variables|Default|GetPaperFlipbook) (Variables|Default|GetbAutoPlay)))

(fn Interact
  (params (PlayerRef :type BP%20Player%20Base%20Object%20Reference))
  (if (not (Variables|Default|GetbeUsed))
    (Variables|Default|SetbeUsed true)
    (CallFunction|UpdateAnimation)))

(fn UpdateAnimation
  (Variables|Default|SetMovementState (select (Variables|Default|GetisFlagOut) "NewEnumerator1" (select (Variables|Default|GetbeUsed) "NewEnumerator0" "NewEnumerator0")))
  (Sprite|SetFlipbook (Variables|Default|GetPaperFlipbook) "/Game/Assets/Flipbooks/Checkpoint_Flag_Out_Flip.Checkpoint_Flag_Out_Flip")
  (Components|Timeline|PlayfromStart (Variables|Default|GetPaperFlipbook)))

(fn SetUnlockLevels
  (params (NextLevelNum :type Integer))
  (bind _gameinstanceref (Variables|References|GetGameInstanceRef))
  (bind _output_get (Variables|Default|SetnextLvlNumb NextLevelNum))
  (if (<= _output_get (Variables|/Game/Blueprints/MainGameInstance.MainGameInstance_C|GetGI_Wrld1LvlsCountOpen _gameinstanceref))
    _
    (else
      (Variables|/Game/Blueprints/MainGameInstance.MainGameInstance_C|SetGI_Wrld1LvlsCountOpen _gameinstanceref _output_get)))
  (return))