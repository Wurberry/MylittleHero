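; BP_InteractiveHealth is an interactive health pickup that restores health to the player who uses it.
; Its Interact function adds HealthValue through the player's AddHealth only when Health is below DefaultHealth, then destroys the actor.
; A player at or above default health leaves the pickup in place.
; The event graph holds only disabled stubs, so all gameplay logic lives in Interact.
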(event EventBeginPlay
  (|CallParentFunction) ; This node is disabled and will not be called.\nDrag off pins to build functionality.
)

(event Collision|EventActorBeginOverlap
  (params (OtherActor :type Actor%20Object%20Reference)))

(event EventTick
  (params (DeltaSeconds :type Float%20%28single-precision%29)))

(fn ConstructionScript
  (|CallParentFunction))

(fn Interact
  (params (PlayerRef :type BP%20Player%20Base%20Object%20Reference))
  (if (< (Variables|/Game/Blueprints/BP_PlayerBase.BP_PlayerBase_C|GetHealth PlayerRef) (Variables|/Game/Blueprints/BP_PlayerBase.BP_PlayerBase_C|GetDefaultHealth PlayerRef))
    (Default|AddHealth PlayerRef (Variables|Default|GetHealthValue))
    (Actor|DestroyActor)))