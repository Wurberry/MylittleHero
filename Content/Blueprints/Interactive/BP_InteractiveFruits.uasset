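; Collectible fruit pickup for a Paper2D game that shows one of eight fruit flipbooks, picked at random on BeginPlay.
; When the player pawn overlaps it, it adds one to the player's fruit level stat widget, sets the player's active level to the current level name and destroys itself.
; A random Delay on Tick toggles flipbook looping, restarting the animation when it turns on, so it animates intermittently.
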(event EventBeginPlay
  ;[1 1 1] BeginPlay
  (|CallParentFunction)
  (CallFunction|SetRandomFlipbook)
  (bind _asbp_player_base (Utilities|Casting|CastToBP_PlayerBase (Game|GetPlayerCharacter 0)))
  (Variables|References|SetPlayerBaseRef _asbp_player_base))

(event Collision|EventActorBeginOverlap
  (params (OtherActor :type Actor%20Object%20Reference))
  ;[1 1 1] OverLap
  (if (== OtherActor (Game|Player|GetPlayerPawn 0))
    (bind _asbp_player_base (Utilities|Casting|CastToBP_PlayerBase (Game|GetPlayerCharacter 0)))
    (Default|UpdateFruitLevelStatWidget _asbp_player_base 1)
    (bind _returnvalue (Game|GetCurrentLevelName true))
    (Variables|/Game/Blueprints/BP_PlayerBase.BP_PlayerBase_C|SetActiveLevel (Variables|References|GetPlayerBaseRef) _returnvalue)
    (Actor|DestroyActor)))

(event EventTick
  (params (DeltaSeconds :type Float%20%28single-precision%29))
  ;[1 1 1] Life Cycle
  (Utilities|FlowControl|Delay (Math|Conversions|ToFloat(Integer) (Math|Float|Truncate (* 10 (Math|Random|RandomFloat)))))
  (Components|Timeline|SetLooping (Variables|Default|GetPaperFlipbook) (not (Variables|Default|GetbAutoPlay)))
  (bind _output_get (Variables|Default|SetbAutoPlay (not (Variables|Default|GetbAutoPlay))))
  (if _output_get
    (Components|Timeline|PlayfromStart (Variables|Default|GetPaperFlipbook))))

(fn ConstructionScript
  (|CallParentFunction))

(fn SetRandomFlipbook
  (switch int (Math|Random|RandomInteger 8)
    (:0
      (LocalVariables|SetselAnim "/Game/Assets/Flipbooks/FruitAppleFlip.FruitAppleFlip"))
    (:1
      (LocalVariables|SetselAnim "/Game/Assets/Flipbooks/FruitBananasFlip.FruitBananasFlip"))
    (:2
      (LocalVariables|SetselAnim "/Game/Assets/Flipbooks/FruitCherriesFlip.FruitCherriesFlip"))
    (:3
      (LocalVariables|SetselAnim "/Game/Assets/Flipbooks/FruitKiwiFlip.FruitKiwiFlip"))
    (:4
      (LocalVariables|SetselAnim "/Game/Assets/Flipbooks/FruitMelonFlip.FruitMelonFlip"))
    (:5
      (LocalVariables|SetselAnim "/Game/Assets/Flipbooks/FruitOrangeFlip.FruitOrangeFlip"))
    (:6
      (LocalVariables|SetselAnim "/Game/Assets/Flipbooks/FruitPineappleFlip.FruitPineappleFlip"))
    (:7
      (LocalVariables|SetselAnim "/Game/Assets/Flipbooks/FruitStrawberryFlip.FruitStrawberryFlip")))
  (Sprite|SetFlipbook (Variables|Default|GetPaperFlipbook) (LocalVariables|GetselAnim)))