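; Bat enemy that patrols horizontally along the world X axis, starting in a random direction.
; Tick feeds constant movement input, and capsule hits on anything but the player with an X normal reverse direction, debounced by a DoOnce with a short delayed reset.
; RotateEnemy faces the sprite by mirroring its X scale.
; Damage reduces clamped health, and at zero the bat calls the parent death logic, destroys itself and sends experience.
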(event OnComponentHit(CapsuleComponent)
  (params (HitComponent :type Primitive%20Component%20Object%20Reference) (OtherActor :type Actor%20Object%20Reference) (OtherComp :type Primitive%20Component%20Object%20Reference) (NormalImpulse :type Vector :default "0, 0, 0") (Hit :type Hit%20Result%20Structure%20%28by%20ref%29))
  ;[0 0 0 1 14] Dont rotation, if hitting player
  (if (!= OtherActor (Game|Player|GetPlayerPawn 0))
    (if (!= (.X (Math|Vector|BreakVector (.normal Hit))) 0.0)
      (Utilities|FlowControl|DoOnce false
        (:Completed
          (bind _output_get (Variables|Default|SetmoveRight (not (Variables|Default|GetmoveRight))))
          (CallFunction|RotateEnemy _output_get)
          (Utilities|FlowControl|Delay 0.2)
          (CallFunction|ResetCheckConstraint))))))

(event Custom|ResetCheckConstraint
  (Utilities|FlowControl|DoOnce false) ; enters at Reset
)

(event EventBeginPlay
  (bind _output_get (Variables|Default|SetmoveRight (Math|Random|RandomBool)))
  (CallFunction|RotateEnemy _output_get)
  (Variables|Default|SetBaseDamage 1.0))

(event EventAnyDamage
  (params (Damage :type Float%20%28single-precision%29) (DamageType :type Damage%20Type%20Object%20Reference) (InstigatedBy :type Controller%20Object%20Reference) (DamageCauser :type Actor%20Object%20Reference))
  (bind _output_get (Variables|Default|SetHealth (Math|Float|Clamp(Float) (- (Variables|Default|GetHealth) Damage) 0.0 (Variables|Default|GetDefaultHealth))))
  (if (and (<= _output_get 0.0) (Variables|Default|GetisLive))
    (CallFunction|EnemyDead)
    (Variables|Default|SetisLive false)
    (CallFunction|SendExp 5)))

(event EventTick
  (params (DeltaSeconds :type Float%20%28single-precision%29))
  (Pawn|Input|AddMovementInput (Math|Vector|MakeVector 1.0 0.0 0.0) (select (Variables|Default|GetmoveRight) 1.0 -1.0) false))

(fn ConstructionScript
  (|CallParentFunction))

(fn EnemyDead
  (|CallParentFunction)
  (Actor|DestroyActor))

(fn RotateEnemy
  (params (Condition :type Boolean))
  (bind _sprite (Variables|Default|GetSprite))
  (bind _returnvalue (Transformation|GetWorldScale _sprite))
  (Transformation|SetWorldScale3D (Variables|Default|GetSprite) (Math|Vector|MakeVector (* (Math|Float|Absolute(Float) (.x _returnvalue)) (select (Variables|Default|GetmoveRight) -1.0 1.0)) (.y _returnvalue) (.z _returnvalue))))