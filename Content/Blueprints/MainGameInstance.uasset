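; Game instance that owns World 1 level progress, the Save1 save slot, menu screens and level switching.
; Init builds 15 BP_WBase_Level objects and fills them from BP_SaveGame, creating the save if missing; saving flattens their strength and fruit values back into arrays.
; World and level numbers are parsed from map names around the underscore.
; Show events create UI widgets, mostly cached, and several set input mode; only World 1 is wired.
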(event Custom|ShowSettings
  ;[1 1 1] Call settings scene
  (Utilities|IsValid (Variables|Widget|GetWBP_Settings)
    (:Is%20Valid
      _)
    (:Is%20Not%20Valid
      (bind _returnvalue (UserInterface|CreateWidget "/Game/Blueprints/GUI/WBP_Settings.WBP_Settings_C" (Game|GetPlayerController 0)))
      (bind _output_get (Variables|Widget|SetWBP_Settings _returnvalue))))
  (UserInterface|Viewport|AddtoViewport _output_get 0))

(event Custom|ShowMainMenu
  (bind _returnvalue (Game|GetPlayerController 0))
  ;[1 1 1] Call main menu and show mouse cursor
  (Utilities|IsValid (Variables|Widget|GetWBP_MainMenu)
    (:Is%20Valid
      _)
    (:Is%20Not%20Valid
      (bind _returnvalue_2 (UserInterface|CreateWidget "/Game/Blueprints/GUI/WBP_MainMenu.WBP_MainMenu_C" _returnvalue))
      (bind _output_get (Variables|Widget|SetWBP_MainMenu _returnvalue_2))))
  (UserInterface|Viewport|AddtoViewport _output_get 0)
  (Variables|/Script/Engine.PlayerController|SetbShowMouseCursor _returnvalue true)
  (Input|SetInputModeUIOnly _returnvalue (Variables|Widget|GetWBP_MainMenu) "LockInFullscreen"))

(event Custom|StopExitAdvert:%20Decline
  ;[1 1 1] Show StopExitAdvert | Hide pause menu
  (Widget|RemovefromParent (Variables|Widget|GetWBP_StopExitAdvert))
  (CallFunction|ShowPauseMenu))

(event Custom|OpenLevel
  (params (WrldNum :type Integer) (LvlNum :type Integer))
  ;[1 1 1] Smart Open Levels
  (switch int WrldNum
    (:0
      (switch int LvlNum
        (:0
          (Game|OpenLevel(byName) "Lvl1_1"))
        (:1
          (Game|OpenLevel(byName) "Lvl1_2"))
        (:2
          (Game|OpenLevel(byName) "Lvl1_3"))
        (:3
          (Game|OpenLevel(byName) "Lvl1_4"))
        (:4
          (Game|OpenLevel(byName) "Lvl1_5"))))))

(event Custom|RestartGame
  ;[1 1 1] Delete + restart level
  (SaveGame|DeleteGameinSlot "Save1")
  (Development|ExecuteConsoleCommand "RestartLevel" 0))

(event Custom|SetLevelsExp
  (params (ExpCount :type Integer) (LvlName :type String) (TypeOfExp :type String))
  ;[1 1 1] SetLevelsExp
  (bind (_wrldnum _lvlnum) (CallFunction|GetWrldLevelfromName LvlName))
  (switch int _wrldnum
    (:1
      (for (_array_element _array_index) (Variables|LevelsArrays|GetLevelsW1Arr)
        (if (== _array_index (- _lvlnum 1))
          (switch string TypeOfExp
            (:Strength
              (Variables|/Game/Levels/World1/BP_WBase_Level.BP_WBase_Level_C|SetStrengthExpCollect _array_element (+ ExpCount (Utilities|Array|Get(acopy) (Variables|LevelsArrays|GetStrengthW1Arr) _array_index)))
              (for _array_element_2 (Variables|LevelsArrays|GetLevelsW1Arr)
                (Utilities|Array|Add (Variables|LevelsArrays|GetStrengthW1Arr) (Variables|/Game/Levels/World1/BP_WBase_Level.BP_WBase_Level_C|GetStrengthExpCollect _array_element_2))))))))))

(event Custom|LoadGame
  ;[1 1 1] LOAD Data from Save slot
  (Development|ExecuteConsoleCommand "RestartLevel" 0)
  ;[1 1 1] Game Instance Init
  (bind _returnvalue (SaveGame|DoesSaveGameExist "Save1"))
  (if _returnvalue
    ;[1 1 1] Load Game functionality
    (bind _returnvalue_2 (SaveGame|LoadGamefromSlot "Save1"))
    (bind _asbp_save_game (Utilities|Casting|CastToBP_SaveGame _returnvalue_2))
    (CallFunction|InitBaseVari)
    (bind (_strenghtw1out _strengthw1arr _fruitscountw1arr) (Default|Load _asbp_save_game))
    (Variables|Default|SetGI_Wrld1LvlsCountOpen _strenghtw1out)
    (for (_array_element _array_index) _strengthw1arr
      (Variables|/Game/Levels/World1/BP_WBase_Level.BP_WBase_Level_C|SetStrengthExpCollect (Utilities|Array|Get(acopy) (Variables|LevelsArrays|GetLevelsW1Arr) _array_index) _array_element))
    (for (_array_element_2 _array_index_2) _fruitscountw1arr
      (Variables|/Game/Levels/World1/BP_WBase_Level.BP_WBase_Level_C|SetFruitsCountCollected (Utilities|Array|Get(acopy) (Variables|LevelsArrays|GetLevelsW1Arr) _array_index_2) _array_element_2))
    (else
      ;[1 1 1] Create save file
      (bind _returnvalue_3 (SaveGame|CreateSaveGameObject "/Game/Blueprints/BP_SaveGame.BP_SaveGame_C"))
      (SaveGame|SaveGametoSlot _returnvalue_3 "Save1")
      (CallFunction|InitBaseVari))))

(event Custom|SaveGameToSlot
  (bind _playerbaseref (Variables|References|GetPlayerBaseRef))
  ;[1 1 1] SAVE Data To Save Slot
  (CallFunction|InitPlayerChar)
  (bind _returnvalue (SaveGame|LoadGamefromSlot "Save1"))
  (bind _asbp_save_game (Utilities|Casting|CastToBP_SaveGame _returnvalue))
  (Utilities|Array|Clear (Variables|LevelsArrays|GetStrengthW1Arr))
  (Utilities|Array|Clear (Variables|LevelsArrays|GetFruitsCountW1))
  (for _array_element (Variables|LevelsArrays|GetLevelsW1Arr)
    (Utilities|Array|Add (Variables|LevelsArrays|GetStrengthW1Arr) (Variables|/Game/Levels/World1/BP_WBase_Level.BP_WBase_Level_C|GetStrengthExpCollect _array_element)))
  (bind _lvlnum (CallFunction|GetWrldLevelfromName (Variables|/Game/Blueprints/BP_PlayerBase.BP_PlayerBase_C|GetActiveLevel _playerbaseref)))
  (for _index (range 0 14)
    (if (== _index _lvlnum)
      (Utilities|Array|Add (Variables|LevelsArrays|GetFruitsCountW1) (Variables|/Game/Blueprints/BP_PlayerBase.BP_PlayerBase_C|GetFruitsCount _playerbaseref))
      (else
        (Utilities|Array|Add (Variables|LevelsArrays|GetFruitsCountW1) (Variables|/Game/Levels/World1/BP_WBase_Level.BP_WBase_Level_C|GetFruitsCountCollected (Utilities|Array|Get(acopy) (Variables|LevelsArrays|GetLevelsW1Arr) _index))))))
  (Default|Save _asbp_save_game (Variables|LevelsArrays|GetStrengthW1Arr) (Variables|Default|GetGI_Wrld1LvlsCountOpen) (Variables|LevelsArrays|GetFruitsCountW1))
  (Utilities|Array|Clear (Variables|LevelsArrays|GetStrengthW1Arr)))

(event Custom|InitBaseVari
  ;[1 1 1] Create save file
  ;;[1 1 1] Init base levels arrays
  (if true
    (for _index (range 0 14)
      (bind _returnvalue (Game|ConstructObjectfromClass "/Game/Levels/World1/BP_WBase_Level.BP_WBase_Level_C" "/Game/Levels/World1/BP_WBase_Level.BP_WBase_Level"))
      (Utilities|Array|Add (Variables|LevelsArrays|GetLevelsW1Arr) _returnvalue))))

(event Custom|InitPlayerChar
  ;[1 1 1] Create save file
  (bind _asbp_player_base (Utilities|Casting|CastToBP_PlayerBase (Game|GetPlayerCharacter 0)))
  (Variables|References|SetPlayerBaseRef _asbp_player_base))

(event Custom|ShowCharactersScreen
  ;[1 1 1] Show Characters Screen
  (Utilities|IsValid (Variables|Widget|GetWBP_CharactersScreen)
    (:Is%20Valid
      _)
    (:Is%20Not%20Valid
      (bind _returnvalue (UserInterface|CreateWidget "/Game/Blueprints/GUI/WBP_Characters.WBP_Characters_C" (Game|GetPlayerController 0)))
      (Variables|Widget|SetWBP_CharactersScreen _returnvalue)))
  (UserInterface|Viewport|AddtoViewport (Variables|Widget|GetWBP_CharactersScreen) 0)
  (for _array_element (Variables|LevelsArrays|GetLevelsW1Arr)
    (Default|UpdatePower (Variables|Widget|GetWBP_CharactersScreen) (Variables|/Game/Levels/World1/BP_WBase_Level.BP_WBase_Level_C|GetStrengthExpCollect _array_element))
    (Default|UpdateAgility (Variables|Widget|GetWBP_CharactersScreen) (Variables|/Game/Levels/World1/BP_WBase_Level.BP_WBase_Level_C|GetAgilityExpCollect _array_element))))

(event Custom|ShowWrld1_LevelsMenu
  (bind _returnvalue (Game|GetPlayerController 0))
  ;[1 1 1] Call W1 levels menu
  (Utilities|IsValid (Variables|Widget|GetWBP_LevelsMenu)
    (:Is%20Valid
      _)
    (:Is%20Not%20Valid
      _))
  (bind _returnvalue_2 (UserInterface|CreateWidget "/Game/Blueprints/GUI/WBP_W1_LevelsMenu.WBP_W1_LevelsMenu_C" (Game|GetPlayerController 0)))
  (bind _output_get (Variables|Widget|SetWBP_LevelsMenu _returnvalue_2))
  (UserInterface|Viewport|AddtoViewport _output_get 0)
  (Input|SetInputModeUIOnly _returnvalue (Variables|Widget|GetWBP_LevelsMenu) "LockInFullscreen")
  (Variables|/Script/Engine.PlayerController|SetbShowMouseCursor _returnvalue true))

(event Custom|ShowLodaingScreen
  (bind _returnvalue (Game|GetPlayerController 0))
  ;[1 1 1] Show loading screen
  (Utilities|IsValid (Variables|Widget|GetWBP_LoadingScreen)
    (:Is%20Valid
      _)
    (:Is%20Not%20Valid
      (bind _returnvalue_2 (UserInterface|CreateWidget "/Game/Blueprints/GUI/WBP_LoadingScreen.WBP_LoadingScreen_C" _returnvalue))
      (bind _output_get (Variables|Widget|SetWBP_LoadingScreen _returnvalue_2))))
  (Variables|/Script/Engine.PlayerController|SetbShowMouseCursor _returnvalue false)
  (UserInterface|Viewport|AddtoViewport _output_get 0))

(event Custom|ShowPauseMenu
  (bind _returnvalue (Game|GetPlayerController 0))
  ;[1 1 1] Show PauseMenu
  (Utilities|IsValid (Variables|Widget|GetWBP_PauseMenu)
    (:Is%20Valid
      _)
    (:Is%20Not%20Valid
      (bind _returnvalue_2 (UserInterface|CreateWidget "/Game/Blueprints/GUI/WBP_PauseMenu.WBP_PauseMenu_C" (Game|GetPlayerController 0)))
      (bind _output_get (Variables|Widget|SetWBP_PauseMenu _returnvalue_2))))
  (UserInterface|Viewport|AddtoViewport _output_get 0)
  (Input|SetInputModeUIOnly _returnvalue (Variables|Widget|GetWBP_PauseMenu) "DoNotLock")
  (Game|SetGamePaused true)
  (Variables|/Script/Engine.PlayerController|SetbShowMouseCursor _returnvalue true))

(event Custom|PauseMenuResume
  (bind _returnvalue (Game|GetPlayerController 0))
  ;[1 1 1] MenuPause Resume in game
  (Widget|RemovefromParent (Variables|Widget|GetWBP_PauseMenu))
  (Game|SetGamePaused false)
  (Input|SetInputModeGameOnly _returnvalue)
  (Variables|/Script/Engine.PlayerController|SetbShowMouseCursor _returnvalue false))

(event Custom|ShowStopExitAdvert
  ;[1 1 1] Show StopExitAdvert | Hide pause menu
  (Utilities|IsValid (Variables|Widget|GetWBP_StopExitAdvert)
    (:Is%20Valid
      _)
    (:Is%20Not%20Valid
      (bind _returnvalue (UserInterface|CreateWidget "/Game/Blueprints/GUI/WBP_StopExitAdvert.WBP_StopExitAdvert_C" (Game|GetPlayerController 0)))
      (bind _output_get (Variables|Widget|SetWBP_StopExitAdvert _returnvalue))))
  (UserInterface|Viewport|AddtoViewport _output_get 0)
  (Widget|RemovefromParent (Variables|Widget|GetWBP_PauseMenu)))

(event Custom|RestartActiveLevel
  ;[1 1 1] Restart Active Level
  (bind _returnvalue (Game|GetCurrentLevelName true))
  (Game|OpenLevel(byName) (Utilities|String|StringToName _returnvalue))
  (Input|SetInputModeGameOnly (Game|GetPlayerController 0)))

(event Custom|StopExitAdvert:%20Accepted
  (params (WorldNum :type Integer))
  ;[1 1 1] Show StopExitAdvert | Hide pause menu
  (switch int WorldNum
    (:0
      (Game|OpenLevel(byName) "W1LevelsMenu"))))

(event Custom|ShowWorldsMenu
  (bind _returnvalue (Game|GetPlayerController 0))
  ;[1 1 1] Call World Set Menu
  (Utilities|IsValid (Variables|Widget|GetWBP_WorldsMenu)
    (:Is%20Valid
      _)
    (:Is%20Not%20Valid
      (bind _returnvalue_2 (UserInterface|CreateWidget "/Game/Blueprints/GUI/WBP_WorldsMenu.WBP_WorldsMenu_C" (Game|GetPlayerController 0)))
      (bind _output_get (Variables|Widget|SetWBP_WorldsMenu _returnvalue_2))))
  (UserInterface|Viewport|AddtoViewport _output_get 0)
  (Input|SetInputModeUIOnly _returnvalue _output_get "LockInFullscreen")
  (Variables|/Script/Engine.PlayerController|SetbShowMouseCursor _returnvalue true))

(event EventInit
  ;[1 1 1] Game Instance Init
  (bind _returnvalue (SaveGame|DoesSaveGameExist "Save1"))
  (if _returnvalue
    ;[1 1 1] Load Game functionality
    (bind _returnvalue_2 (SaveGame|LoadGamefromSlot "Save1"))
    (bind _asbp_save_game (Utilities|Casting|CastToBP_SaveGame _returnvalue_2))
    (CallFunction|InitBaseVari)
    (bind (_strenghtw1out _strengthw1arr _fruitscountw1arr) (Default|Load _asbp_save_game))
    (Variables|Default|SetGI_Wrld1LvlsCountOpen _strenghtw1out)
    (for (_array_element _array_index) _strengthw1arr
      (Variables|/Game/Levels/World1/BP_WBase_Level.BP_WBase_Level_C|SetStrengthExpCollect (Utilities|Array|Get(acopy) (Variables|LevelsArrays|GetLevelsW1Arr) _array_index) _array_element))
    (for (_array_element_2 _array_index_2) _fruitscountw1arr
      (Variables|/Game/Levels/World1/BP_WBase_Level.BP_WBase_Level_C|SetFruitsCountCollected (Utilities|Array|Get(acopy) (Variables|LevelsArrays|GetLevelsW1Arr) _array_index_2) _array_element_2))
    (else
      ;[1 1 1] Create save file
      (bind _returnvalue_3 (SaveGame|CreateSaveGameObject "/Game/Blueprints/BP_SaveGame.BP_SaveGame_C"))
      (SaveGame|SaveGametoSlot _returnvalue_3 "Save1")
      (CallFunction|InitBaseVari))))

(fn GetWrldLevelfromName
  (params (LvlName :type String))
  (bind _returnvalue (Utilities|String|FindSubstring LvlName "_"))
  (bind _returnvalue_2 (+ _returnvalue 1))
  (return (Math|Conversions|ToInteger(Byte) (Utilities|String|GetSubstring LvlName (- _returnvalue 1))) (Math|Conversions|ToInteger(Byte) (Utilities|String|GetSubstring LvlName _returnvalue_2 (- (Utilities|String|Len LvlName) _returnvalue_2)))))

(fn UpdateLevelsExpInfo
  ;[0 0 0] The same for other worlds or stats
  (for _array_element (Variables|LevelsArrays|GetLevelsW1Arr)
    (Variables|Stats|SetStrengthExpCount (+ (Variables|/Game/Levels/World1/BP_WBase_Level.BP_WBase_Level_C|GetStrengthExpCollect _array_element) (Variables|Stats|GetStrengthExpCount)))
    (Development|PrintString "Hello")))