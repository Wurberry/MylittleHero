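; Player projectile that travels horizontally along the X axis and damages what it hits.
; On BeginPlay it moves to the player pawn's location and copies the horizontal direction value from BP_PlayerBase.
; Tick offsets its X position by that direction, speed and delta time, without physics or a movement component.
; The first actor overlap, with no filtering by actor type, applies damage and destroys the bullet.
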(event EventBeginPlay
  (bind _returnvalue (Game|Player|GetPlayerPawn 0))
  (bind _asplayer_base (Utilities|Casting|CastToBP_PlayerBase _returnvalue))
  (bind _output_get (Variables|Default|Setplr _asplayer_base))
  (Variables|Default|SetdirMovRight (Variables|/Game/Blueprints/BP_PlayerBase.BP_PlayerBase_C|Getdirxright _output_get))
  (Transformation|SetActorLocation (Transformation|GetActorLocation _returnvalue) false false))

(event Collision|EventActorBeginOverlap
  (params (OtherActor :type Actor%20Object%20Reference))
  (Game|Damage|ApplyDamage OtherActor (Variables|Default|Getdmg) 0 0)
  (Actor|DestroyActor))

(event EventTick
  (params (DeltaSeconds :type Float%20%28single-precision%29))
  (bind _returnvalue (Transformation|GetActorLocation))
  (bind (_x _y _z) (Math|Vector|BreakVector _returnvalue))
  (Transformation|SetActorLocation (Math|Vector|MakeVector (+ (* (Math|Conversions|ToFloat(Integer) (Variables|Default|GetdirMovRight)) (Variables|Default|Getspeed) DeltaSeconds) _x) _y _z) false false))

(fn ConstructionScript)